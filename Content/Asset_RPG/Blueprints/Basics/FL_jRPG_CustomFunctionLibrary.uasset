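; Blueprint function library of shared helpers for the jRPG game, mostly for UI display.
; Select nodes map stat, item, subtype, rarity and action enums to display text, default item icons or rarity colors.
; Data table lookups return item and action display names and the clamped XP remaining to the next level.
; ChangeMap stores the map and spawn point names on the custom GameInstance, then opens the level by name.
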(fn `ActionTypeToText`
  (params (ActionType :type "/Game/Asset_RPG/Enumerations/E_jRPG_ActionType Enum" :default "NewEnumerator6"))
  (returns (Text :type Text))
  (return (select `/Game/Asset_RPG/Enumerations/E_jRPG_ActionType` ActionType :`NewEnumerator0` "Attack" :`NewEnumerator1` "Defend" :`NewEnumerator2` "Items" :`NewEnumerator5` "Flee" :`NewEnumerator3` "Magic" :`NewEnumerator4` "Moves" :`NewEnumerator7` "Deathblow" :!type "Text")))

(fn `ChangeMap`
  (params (MapName :type Name) (SpawnPointName :type Name))
  (bind _asbp_j_rpg_gi_custom (cast `/Game/Asset_RPG/Blueprints/Basics/BP_jRPG_GI_Custom` (`GameplayStatics.GetGameInstance` null)))
  (set `/Game/Asset_RPG/Blueprints/Basics/BP_jRPG_GI_Custom.WorldMapSpawnPointName` SpawnPointName _asbp_j_rpg_gi_custom)
  (set `/Game/Asset_RPG/Blueprints/Basics/BP_jRPG_GI_Custom.WorldMapName` MapName _asbp_j_rpg_gi_custom)
  (`GameplayStatics.OpenLevel` null MapName))

(fn `GetActionDisplayName`
  (params (ActionHardcodedName :type Name))
  (returns (ActionDisplayName :type Text))
  (bind _returnvalue (`|GetDataTableRow` "/Game/Asset_RPG/Datatables/DT_jRPG_Actions.DT_jRPG_Actions" ActionHardcodedName)
    (:`then`
      (return (`.DisplayName_5_625DFD5A419E4C6CC34A148337F3099D` (break `/Game/Asset_RPG/Structures/Actions/S_jRPG_Action` _returnvalue))))))

(fn `GetExperienceNeededToNextLevel`
  (params (CurrentLevel :type Integer) (CurrentXP :type Integer))
  (returns (XPtoNextLevel :type Integer))
  (bind _returnvalue (`|GetDataTableRow` "/Game/Asset_RPG/Datatables/DT_jRPG_Levels.DT_jRPG_Levels" (`KismetStringLibrary.Conv_StringToName` (`KismetStringLibrary.Conv_IntToString` (+ CurrentLevel 1))))
    (:`then`
      (bind _experienceneededtoreachthislevel (break `/Game/Asset_RPG/Structures/S_jRPG_Level` _returnvalue))
      (return (`KismetMathLibrary.Clamp` (- _experienceneededtoreachthislevel CurrentXP) 0 _experienceneededtoreachthislevel)))))

(fn `GetItemDisplayName`
  (params (ItemHardcodedName :type Name))
  (returns (ItemDisplayName :type Text))
  (bind _returnvalue (`|GetDataTableRow` "/Game/Asset_RPG/Datatables/DT_jRPG_Items.DT_jRPG_Items" ItemHardcodedName)
    (:`then`
      (return (`.ItemDisplayName_29_41C0C54E4A55598869C84CA3B5B5DECA` (break `/Game/Asset_RPG/Structures/S_jRPG_Item_StaticData` _returnvalue))))))

(fn `ItemSubypeToText`
  (params (ItemSubtype :type "/Game/Asset_RPG/Enumerations/E_jRPG_ItemSubtype Enum" :default "NewEnumerator3"))
  (returns (Text :type Text))
  (return (select `/Game/Asset_RPG/Enumerations/E_jRPG_ItemSubtype` ItemSubtype :`NewEnumerator0` "Sword" :`NewEnumerator1` "Staff" :`NewEnumerator2` "Bow" :`NewEnumerator4` "Axe" :`NewEnumerator8` "Dagger" :`NewEnumerator5` "Heavy Protection" :`NewEnumerator6` "Leather Protection" :`NewEnumerator7` "Robe Protection" :`NewEnumerator9` "Ring" :`NewEnumerator10` "Necklace" :`NewEnumerator11` "Medicine" :!type "Text")))

(fn `ItemTypeToImage`
  (params (ItemType :type "/Game/Asset_RPG/Enumerations/E_jRPG_ItemType Enum" :default "NewEnumerator6"))
  (returns (Image :type "Texture2D Object Reference"))
  (return (select `/Game/Asset_RPG/Enumerations/E_jRPG_ItemType` ItemType :`NewEnumerator0` "/Game/Asset_RPG/Demo/Icons/I_UI_DefaultWeapon.I_UI_DefaultWeapon" :`NewEnumerator1` "/Game/Asset_RPG/Demo/Icons/I_UI_DefaultArmor.I_UI_DefaultArmor" :`NewEnumerator2` "/Game/Asset_RPG/Demo/Icons/I_UI_DefaultHelmet.I_UI_DefaultHelmet" :`NewEnumerator3` "/Game/Asset_RPG/Demo/Icons/I_UI_DefautGloves.I_UI_DefautGloves" :`NewEnumerator4` "/Game/Asset_RPG/Demo/Icons/I_UI_DefaultBoots.I_UI_DefaultBoots" :`NewEnumerator5` "/Game/Asset_RPG/Demo/Icons/I_UI_DefaultRing.I_UI_DefaultRing" :!type "Texture2D Object Reference")))

(fn `ItemTypeToText`
  (params (ItemType :type "/Game/Asset_RPG/Enumerations/E_jRPG_ItemType Enum" :default "NewEnumerator6"))
  (returns (Text :type Text))
  (return (select `/Game/Asset_RPG/Enumerations/E_jRPG_ItemType` ItemType :`NewEnumerator0` "Weapon" :`NewEnumerator1` "Armor" :`NewEnumerator2` "Helmet" :`NewEnumerator3` "Gloves" :`NewEnumerator4` "Boots" :`NewEnumerator5` "Accessory" :`NewEnumerator7` "Potion" :!type "Text")))

(fn `RarityToColor`
  (params (Rarity :type "/Game/Asset_RPG/Enumerations/E_jRPG_ItemRarity Enum" :default "NewEnumerator5"))
  (returns (LinearColor :type "LinearColor Structure"))
  (return (select `/Game/Asset_RPG/Enumerations/E_jRPG_ItemRarity` Rarity :`NewEnumerator5` (struct :`A` 1.0) :`NewEnumerator0` (struct :`A` 1.0) :`NewEnumerator1` (struct :`G` 1.0 :`B` 1.0 :`A` 1.0) :`NewEnumerator2` (struct :`G` 1.0 :`A` 1.0) :`NewEnumerator3` (struct :`R` 1.0 :`B` 1.0 :`A` 1.0) :`NewEnumerator4` (struct :`R` 1.0 :`A` 1.0) :`NewEnumerator6` (struct :`R` 1.0 :`G` 1.0 :`A` 1.0) :!type "LinearColor Structure")))

(fn `RarityToText`
  (params (Rarity :type "/Game/Asset_RPG/Enumerations/E_jRPG_ItemRarity Enum" :default "NewEnumerator5"))
  (returns (Text :type Text))
  (return (select `/Game/Asset_RPG/Enumerations/E_jRPG_ItemRarity` Rarity :`NewEnumerator0` "Common" :`NewEnumerator1` "Magic" :`NewEnumerator2` "Rare" :`NewEnumerator3` "Epic" :`NewEnumerator4` "Artifact" :`NewEnumerator6` "Legendary" :!type "Text")))

(fn `StatTypeToText`
  (params (StatType :type "/Game/Asset_RPG/Enumerations/E_jRPG_StatType Enum" :default "NewEnumerator0"))
  (returns (Text :type Text))
  (return (select `/Game/Asset_RPG/Enumerations/E_jRPG_StatType` StatType :`NewEnumerator1` "HP" :`NewEnumerator2` "MP" :`NewEnumerator3` "Power" :`NewEnumerator4` "Defence" :`NewEnumerator5` "Crit Rate" :`NewEnumerator6` "Crit Power" :`NewEnumerator7` "Initiative" :`NewEnumerator8` "Evasion" :!type "Text")))