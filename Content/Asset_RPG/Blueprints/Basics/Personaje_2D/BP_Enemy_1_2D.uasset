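; 2D rat enemy for turn-based RPG battles, with a simple AI attack and a death sequence.
; On its turn it announces the attack, ends its turn, plays the attack animation, then damages a random player character using its own stats and spawns an impact effect.
; Delays pace the action before it resumes the battle and returns to idle.
; On death it plays a death animation, then notifies the battle manager.
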(event `self.PerformActionByAI`
  (bind _battlemanagerreference (`self.BattleManagerReference`))
  (bind _playercharacters (`/Game/Asset_RPG/Blueprints/Components/AC_jRPG_BattleManager.PlayerCharacters` (`self.BattleManagerReference`)))
  (bind _characterstats (`/Game/Asset_RPG/Blueprints/Components/AC_jRPG_CharacterBattleStats.CharacterStats` (`self.AC_jRPG_CharacterBattleStats`)))
  (`/Game/Asset_RPG/Blueprints/Components/AC_jRPG_BattleManager.ShowBattleTooltip` _battlemanagerreference (`|FormatText` "{name} attacks" (`/Game/Asset_RPG/Blueprints/Components/AC_jRPG_CharacterBattleStats.CharacterDisplayName` (`self.AC_jRPG_CharacterBattleStats`))))
  (`/Game/Asset_RPG/Blueprints/Components/AC_jRPG_BattleManager.EndCharacterTurn` _battlemanagerreference 1000.0)
  (`KismetSystemLibrary.Delay` 0.25)
  (bind _animationlength (`PaperZDAnimInstance.K2_PlayAnimationOverride` (`PaperZDAnimationComponent.AnimInstance` (`self.AnimationComponent`)) "/Game/Asset_RPG/Blueprints/Basics/Personaje_2D/Sprites/Enemigos_2D/Ratas/AnimSequences/Ataque_Rata.Ataque_Rata" "DefaultSlot" 1.0 0.0))
  (`KismetSystemLibrary.Delay` _animationlength)
  (bind _output_get (set `self.Targeted` (`|GetArrayItem` _playercharacters (`KismetMathLibrary.RandomIntegerInRange` 0 (- (`KismetArrayLibrary.Array_Length` _playercharacters) 1)))))
  (`/Game/Asset_RPG/Blueprints/Components/AC_jRPG_CharacterBattleStats.ReceiveDamage` (`/Game/Asset_RPG/Blueprints/Basics/Personaje_2D/BP_Character_Battle_Base_2D.AC_jRPG_CharacterBattleStats` _output_get) (`BlueprintMapLibrary.Map_Find` _characterstats "NewEnumerator3") (`BlueprintMapLibrary.Map_Find` _characterstats "NewEnumerator5") (`BlueprintMapLibrary.Map_Find` _characterstats "NewEnumerator6"))
  (`GameplayStatics.SpawnEmitterAtLocation` "/Game/Asset_RPG/Demo/VFX/Particles/Impact/P_Impact_Generic.P_Impact_Generic" (`self.K2_GetActorLocation` _output_get))
  (`KismetSystemLibrary.Delay` 1.0)
  (`/Game/Asset_RPG/Blueprints/Components/AC_jRPG_BattleManager.ResumeBattle` (`self.BattleManagerReference`))
  (`PaperZDPlaySlotOverrideAction.PlayAnimationOverrideWithCallbacks` (`PaperZDAnimationComponent.AnimInstance` (`self.AnimationComponent`)) "/Game/Asset_RPG/Blueprints/Basics/Personaje_2D/Sprites/Enemigos_2D/Ratas/AnimSequences/Idle_rata.Idle_rata"))

(event `/Game/Asset_RPG/Blueprints/Interfaces/BPI_BattleCommunication.OnDeath`
  (set `self.Dead?` true)
  (`PaperZDPlaySlotOverrideAction.PlayAnimationOverrideWithCallbacks` (`PaperZDAnimationComponent.AnimInstance` (`self.AnimationComponent`)) "/Game/Asset_RPG/Blueprints/Basics/Personaje_2D/Sprites/Enemigos_2D/Ratas/AnimSequences/Dead_rata.Dead_rata"
    (:`OnCompleted`
      (`KismetSystemLibrary.Delay` 0.2)
      (bind _battlemanagerreference (`self.BattleManagerReference`)
        (:`then`
          (`/Game/Asset_RPG/Blueprints/Components/AC_jRPG_BattleManager.OnEnemyKilled` _battlemanagerreference self))
        (:`else`)))))

(fn `UserConstructionScript`
  (`parent.UserConstructionScript`))