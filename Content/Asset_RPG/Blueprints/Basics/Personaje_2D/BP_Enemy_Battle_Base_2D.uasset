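; Base Blueprint for a 2D battle enemy that handles its death and reports it to the battle manager.
; OnDeath sets the Dead flag and plays the Dead_rata animation as an override on the animation instance.
; Both the immediate and Completed outputs of that call feed a 0.2-second delay, then OnEnemyKilled is called on the battle manager if valid.
; BeginPlay, overlap and construction only call the parent.
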(event `self.ReceiveBeginPlay`
  (`parent.ReceiveBeginPlay`))

(event `self.ReceiveActorBeginOverlap`
  (params (OtherActor :type "Actor Object Reference"))
  (`parent.ReceiveActorBeginOverlap` OtherActor))

(event `/Game/Asset_RPG/Blueprints/Interfaces/BPI_BattleCommunication.OnDeath`
  (set `self.Dead?` true)
  (`PaperZDPlaySlotOverrideAction.PlayAnimationOverrideWithCallbacks` (`PaperZDAnimationComponent.AnimInstance` (`self.AnimationComponent`)) "/Game/Asset_RPG/Blueprints/Basics/Personaje_2D/Sprites/Enemigos_2D/Ratas/AnimSequences/Dead_rata.Dead_rata"
    (:`then`
      _)
    (:`OnCompleted`
      _))
  (`KismetSystemLibrary.Delay` 0.2)
  (bind _battlemanagerreference (`self.BattleManagerReference`)
    (:`then`
      (`/Game/Asset_RPG/Blueprints/Components/AC_jRPG_BattleManager.OnEnemyKilled` _battlemanagerreference self))
    (:`else`)))

(fn `UserConstructionScript`
  (`parent.UserConstructionScript`))