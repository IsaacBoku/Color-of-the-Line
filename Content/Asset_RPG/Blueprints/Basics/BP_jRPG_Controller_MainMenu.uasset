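; Player controller for the jRPG main menu, which sets up menu input and shows the main menu widget.
; On BeginPlay it creates the menu widget with the save manager component passed in, then refreshes that manager's load slots.
; If gamepad controls are enabled, it hides the cursor and activates main-menu gamepad navigation.
; D-pad, face button, shoulder and trigger presses forward directly to the gamepad controls component.
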(event `self.ReceiveBeginPlay`
  (`WidgetBlueprintLibrary.SetInputMode_GameAndUIEx` self null "DoNotLock" false) ; Set up proper input
  (bind _returnvalue (`|CreateWidget` "/Game/Asset_RPG/Widgets/MainMenu/WBP_jRPG_MainMenu.WBP_jRPG_MainMenu_C" null (`self.AC_jRPG_SaveManager`)))
  (bind _output_get (set `self.MainMenuWidgetReference` _returnvalue))
  (`UserWidget.AddToViewport` _output_get 0)
  (`/Game/Asset_RPG/Blueprints/Components/AC_jRPG_SaveManager.RefreshLoadSlots` (`self.AC_jRPG_SaveManager`))
  (if (`/Game/Asset_RPG/Blueprints/Components/AC_jRPG_GamepadControls.GamepadControlsEnabled?` (`self.AC_jRPG_GamepadControls`))
    (set `self.bShowMouseCursor` false)
    (`/Game/Asset_RPG/Blueprints/Components/AC_jRPG_GamepadControls.ActivateGamepadControls - MainMenu` (`self.AC_jRPG_GamepadControls`))))

(event `InputAction|D-PadUp` :paused true
  (params (Key :type "Key Structure"))
  (:`Pressed`
    (`/Game/Asset_RPG/Blueprints/Components/AC_jRPG_GamepadControls.D-PadUpPressed` (`self.AC_jRPG_GamepadControls`))))

(event `InputAction|D-PadDown` :paused true
  (params (Key :type "Key Structure"))
  (:`Pressed`
    (`/Game/Asset_RPG/Blueprints/Components/AC_jRPG_GamepadControls.D-PadDownPressed` (`self.AC_jRPG_GamepadControls`))))

(event `InputAction|D-PadRight` :paused true
  (params (Key :type "Key Structure"))
  (:`Pressed`
    (`/Game/Asset_RPG/Blueprints/Components/AC_jRPG_GamepadControls.D-PadRightPressed` (`self.AC_jRPG_GamepadControls`))))

(event `InputAction|D-PadLeft` :paused true
  (params (Key :type "Key Structure"))
  (:`Pressed`
    (`/Game/Asset_RPG/Blueprints/Components/AC_jRPG_GamepadControls.D-PadLeftPressed` (`self.AC_jRPG_GamepadControls`))))

(event `InputAction|AcceptButton` :paused true
  (params (Key :type "Key Structure"))
  (:`Pressed`
    (`/Game/Asset_RPG/Blueprints/Components/AC_jRPG_GamepadControls.FaceButtonBottomPressed` (`self.AC_jRPG_GamepadControls`))))

(event `InputAction|CancelButton` :paused true
  (params (Key :type "Key Structure"))
  (:`Pressed`
    (`/Game/Asset_RPG/Blueprints/Components/AC_jRPG_GamepadControls.FaceButtonRightPressed` (`self.AC_jRPG_GamepadControls`))))

(event `InputAction|SelectButton` :paused true
  (params (Key :type "Key Structure"))
  (:`Pressed`
    (`/Game/Asset_RPG/Blueprints/Components/AC_jRPG_GamepadControls.FaceButtonLeftPressed` (`self.AC_jRPG_GamepadControls`))))

(event `InputAction|DiscardButton` :paused true
  (params (Key :type "Key Structure"))
  (:`Pressed`
    (`/Game/Asset_RPG/Blueprints/Components/AC_jRPG_GamepadControls.FaceButtonTopPressed` (`self.AC_jRPG_GamepadControls`))))

(event `InputAction|ShoulderRight` :paused true
  (params (Key :type "Key Structure"))
  (:`Pressed`
    (`/Game/Asset_RPG/Blueprints/Components/AC_jRPG_GamepadControls.ShoulderRightPressed` (`self.AC_jRPG_GamepadControls`))))

(event `InputAction|TriggerRight` :paused true
  (params (Key :type "Key Structure"))
  (:`Pressed`
    (`/Game/Asset_RPG/Blueprints/Components/AC_jRPG_GamepadControls.TriggerRightPressed` (`self.AC_jRPG_GamepadControls`))))

(event `InputAction|ShoulderLeft`
  (params (Key :type "Key Structure"))
  (:`Pressed`
    (`/Game/Asset_RPG/Blueprints/Components/AC_jRPG_GamepadControls.ShoulderLeftPressed` (`self.AC_jRPG_GamepadControls`))))

(event `InputAction|TriggerLeft`
  (params (Key :type "Key Structure"))
  (:`Pressed`
    (`/Game/Asset_RPG/Blueprints/Components/AC_jRPG_GamepadControls.TriggerLeftPressed` (`self.AC_jRPG_GamepadControls`))))

(fn `UserConstructionScript`)