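; Camera path actor for jRPG battles that defines a procedural spline and a focus point for a dynamic camera.
; The Construction Script builds a loop or spiral from trigonometry, adds direction arrows at each point and applies the initial path rotation.
; It also places a preview camera at the path start, aimed at the focus point.
; Getters return the world focus point and path location, whose Time input is really spline distance.
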(fn `GetCameraFocusPoint`
  (returns (FocusLocation :type "Vector Structure"))
  (return (+ (`self.K2_GetActorLocation`) (`self.CameraFocusPoint`))))

(fn `GetPathLocationAtDistance`
  (params (Time :type "Float (double-precision)"))
  (returns (World :type "Vector Structure"))
  (return (`SplineComponent.GetLocationAtDistanceAlongSpline` (`self.Spline`) Time "World")))

(fn `UserConstructionScript`
  (bind _loopradius (`self.LoopRadius`))
  (bind _spiralradius (`self.SpiralRadius`))
  (`|ExecutionSequence`
    (:`then_0`
      (switch `/Game/Asset_RPG/Enumerations/E_jRPG_CameraPathType` (`self.PathType`)
        (:`NewEnumerator0`
          ;[1 1 1] Loop Type set up
          (`SplineComponent.SetClosedLoop` (`self.Spline`) (`self.LoopClosed`) true)
          (`SplineComponent.ClearSplinePoints` (`self.Spline`) true)
          (for _index (range 1 (+ (`self.PointsAmount`) 1))
            (bind _returnvalue (* _index (/ 360.0 (`KismetMathLibrary.Conv_IntToDouble` (`self.PointsAmount`)))))
            (`SplineComponent.AddSplinePoint` (`self.Spline`) (`KismetMathLibrary.MakeVector` (* _loopradius (`KismetMathLibrary.DegCos` _returnvalue)) (* _loopradius (`KismetMathLibrary.DegSin` _returnvalue))) "Local" true)))
        (:`NewEnumerator1`
          ;[1 1 1] Spiral Type set up
          (`SplineComponent.SetClosedLoop` (`self.Spline`) false true)
          (`SplineComponent.ClearSplinePoints` (`self.Spline`) true)
          (for _index_2 (range 1 (+ (`KismetMathLibrary.Round` (* (`self.PointsAmount`) (`self.SpiralLength`))) 1))
            (bind _returnvalue_2 (* _index_2 (/ 360.0 (`KismetMathLibrary.Conv_IntToDouble` (`self.PointsAmount`)))))
            (`SplineComponent.AddSplinePoint` (`self.Spline`) (`KismetMathLibrary.MakeVector` (* _spiralradius (`KismetMathLibrary.DegCos` _returnvalue_2)) (* _spiralradius (`KismetMathLibrary.DegSin` _returnvalue_2)) (* (/ (`KismetMathLibrary.Conv_IntToDouble` _index_2) (`KismetMathLibrary.Conv_IntToDouble` (`self.PointsAmount`))) (`self.SpiralOffset`))) "Local" true))))
      ;[1 1 1] Add arrows along spline
      (for _index_3 (range (`SplineComponent.GetNumberOfSplinePoints` (`self.Spline`)))
        (`AddComponent|NODE_AddArrowComponent-0` :`RelativeTransform` (`KismetMathLibrary.MakeTransform` (`SplineComponent.GetLocationAtSplinePoint` (`self.Spline`) _index_3 "Local") (`SplineComponent.GetRotationAtSplinePoint` (`self.Spline`) _index_3 "Local") (0.5 0.5 0.5)))))
    (:`then_1`
      (`SceneComponent.K2_SetRelativeRotation` (`self.Spline`) (`self.PathInitialRotation`) false false))
    (:`then_2`
      (`SceneComponent.K2_SetRelativeLocation` (`self.PreviewCamera`) (`SplineComponent.GetLocationAtTime` (`self.Spline`) 0.0 "Local" false) false false)
      (`SceneComponent.K2_SetWorldRotation` (`self.PreviewCamera`) (`KismetMathLibrary.FindLookAtRotation` (`SceneComponent.K2_GetComponentLocation` (`self.PreviewCamera`)) (+ (`self.K2_GetActorLocation`) (`self.CameraFocusPoint`))) false false))))