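; Dialogue component for the character Molly, defining her conversation on top of a parent dialogue system.
; It switches on the active tree branch: the default greeting plays with audio and an idle animation, then sets the GivenCheese branch.
; The Given Cheese branch picks one of two random replies, then clears progress and closes the conversation.
; An unconnected give-or-keep beer choice and other stray nodes never run.
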(fn `Dialogue`
  (`parent.Dialogue`)
  (switch `name` (`self.ActiveTreeBranch`)
    (:`Default`
      (bind _state (`self.AddDialogue` "Molly" "How are you, little guy?" (`|MakeArray`) "/Engine/VREditor/Sounds/UI/Click_on_Button_Cue.Click_on_Button_Cue" "/Game/Asset_RPG/Blueprints/Basics/Personaje_2D/Sprites/Molly_NPC/AnimSequences/Idle.Idle"))
      (switch `/Game/Dialogue_System/E_DialogueState` _state
        (:`NewEnumerator0`
          (`self.SetDialogueBranch` "GivenCheese")
          (`self.CloseConversation`))))
    (:`GivenCheese`
      (bind _state_2 (`self.AddDialogue` "Molly" (select `int` (`KismetMathLibrary.RandomIntegerInRange` 0 1) :`0` "Your much" :`1` "No no" :!type "Text") (`|MakeArray`)))
      (switch `/Game/Dialogue_System/E_DialogueState` _state_2
        (:`NewEnumerator0`
          (`self.ClearDialogueProgress`)
          (`self.CloseConversation`))))))