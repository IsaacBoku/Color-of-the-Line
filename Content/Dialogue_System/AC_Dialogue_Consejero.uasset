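; Dialogue component for the Consejero NPC, who catches Charlie with a book and offers to reveal how one kingdom split in two.
; The Dialogue override is a linear chain of nested AddDialogue calls with single-choice replies, advanced through each node's State and OptionIndex.
; The last line's Update state shows the WBP_Cinematica widget, starts the media player and loads Map_Final after a fixed 90-second delay.
; Its Pass Through state sets the "Normal" branch and closes the conversation.
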(event `Delay`
  (`KismetSystemLibrary.Delay` 90.0)
  (`GameplayStatics.OpenLevel` "Map_Final"))

(fn `Dialogue`
  (`parent.Dialogue`)
  (switch `name` (`self.ActiveTreeBranch`)
    (:`Default`
      (bind (_state _optionindex) (`self.AddDialogue` "Consejero" "Hey, you, stop right there!" (`|MakeArray` "(Oh oh, I think they caught me…)" :!type "Text") "/Engine/VREditor/Sounds/UI/Click_on_Button_Cue.Click_on_Button_Cue" "/Game/Asset_RPG/Blueprints/Basics/Personaje_2D/Sprites/Molly_NPC/AnimSequences/Idle.Idle"))
      (switch `/Game/Dialogue_System/E_DialogueState` _state
        (:`NewEnumerator0`
          (switch `int` _optionindex
            (:`0`
              (bind _state_2 (`self.AddDialogue` "Charlie" "This isn't what it looks like!" (`|MakeArray`) "/Engine/VREditor/Sounds/UI/Click_on_Button_Cue.Click_on_Button_Cue" "/Game/Asset_RPG/Blueprints/Basics/Personaje_2D/Sprites/Molly_NPC/AnimSequences/Idle.Idle"))
              (switch `/Game/Dialogue_System/E_DialogueState` _state_2
                (:`NewEnumerator0`
                  (bind _state_3 (`self.AddDialogue` "Charlie" "I didn’t mean to steal the book!" (`|MakeArray`) "/Engine/VREditor/Sounds/UI/Click_on_Button_Cue.Click_on_Button_Cue" "/Game/Asset_RPG/Blueprints/Basics/Personaje_2D/Sprites/Molly_NPC/AnimSequences/Idle.Idle"))
                  (switch `/Game/Dialogue_System/E_DialogueState` _state_3
                    (:`NewEnumerator0`
                      (bind (_state_4 _optionindex_2) (`self.AddDialogue` "???" "(Although I WAS going to take it after seeing it, truth be told…)" (`|MakeArray`) "/Engine/VREditor/Sounds/UI/Click_on_Button_Cue.Click_on_Button_Cue" "/Game/Asset_RPG/Blueprints/Basics/Personaje_2D/Sprites/Molly_NPC/AnimSequences/Idle.Idle"))
                      (switch `/Game/Dialogue_System/E_DialogueState` _state_4
                        (:`NewEnumerator0`
                          (switch `int` _optionindex_2
                            (:`0`
                              (bind (_state_5 _optionindex_3) (`self.AddDialogue` "???" "Well, and here I was thinking something interesting would finally happen after being here for so long…" (`|MakeArray` "What do you mean?" :!type "Text") "/Engine/VREditor/Sounds/UI/Click_on_Button_Cue.Click_on_Button_Cue" "/Game/Asset_RPG/Blueprints/Basics/Personaje_2D/Sprites/Molly_NPC/AnimSequences/Idle.Idle"))
                              (switch `/Game/Dialogue_System/E_DialogueState` _state_5
                                (:`NewEnumerator0`
                                  (switch `int` _optionindex_3
                                    (:`0`
                                      (bind (_state_6 _optionindex_4) (`self.AddDialogue` "???" "I’ve been safekeeping this book for a really long time." (`|MakeArray`) "/Engine/VREditor/Sounds/UI/Click_on_Button_Cue.Click_on_Button_Cue" "/Game/Asset_RPG/Blueprints/Basics/Personaje_2D/Sprites/Molly_NPC/AnimSequences/Idle.Idle"))
                                      (switch `/Game/Dialogue_System/E_DialogueState` _state_6
                                        (:`NewEnumerator0`
                                          (switch `int` _optionindex_4
                                            (:`0`
                                              (bind (_state_7 _optionindex_5) (`self.AddDialogue` "???" "Ever since “that” happened…" (`|MakeArray` "“That”? What are you talking about?" :!type "Text") "/Engine/VREditor/Sounds/UI/Click_on_Button_Cue.Click_on_Button_Cue" "/Game/Asset_RPG/Blueprints/Basics/Personaje_2D/Sprites/Molly_NPC/AnimSequences/Idle.Idle"))
                                              (switch `/Game/Dialogue_System/E_DialogueState` _state_7
                                                (:`NewEnumerator0`
                                                  (switch `int` _optionindex_5
                                                    (:`0`
                                                      (bind (_state_8 _optionindex_6) (`self.AddDialogue` "???" "Whoops, I forgot." (`|MakeArray`) "/Engine/VREditor/Sounds/UI/Click_on_Button_Cue.Click_on_Button_Cue" "/Game/Asset_RPG/Blueprints/Basics/Personaje_2D/Sprites/Molly_NPC/AnimSequences/Idle.Idle"))
                                                      (switch `/Game/Dialogue_System/E_DialogueState` _state_8
                                                        (:`NewEnumerator0`
                                                          (switch `int` _optionindex_6
                                                            (:`0`
                                                              (bind (_state_9 _optionindex_7) (`self.AddDialogue` "???" "Since it happened so long ago it’s only normal people don’t remember what occurred." (`|MakeArray` "I have no idea what you’re talking about, spit it out already!" :!type "Text") "/Engine/VREditor/Sounds/UI/Click_on_Button_Cue.Click_on_Button_Cue" "/Game/Asset_RPG/Blueprints/Basics/Personaje_2D/Sprites/Molly_NPC/AnimSequences/Idle.Idle"))
                                                              (switch `/Game/Dialogue_System/E_DialogueState` _state_9
                                                                (:`NewEnumerator0`
                                                                  (switch `int` _optionindex_7
                                                                    (:`0`
                                                                      (bind (_state_10 _optionindex_8) (`self.AddDialogue` "???" "The separation of the universe…" (`|MakeArray`) "/Engine/VREditor/Sounds/UI/Click_on_Button_Cue.Click_on_Button_Cue" "/Game/Asset_RPG/Blueprints/Basics/Personaje_2D/Sprites/Molly_NPC/AnimSequences/Idle.Idle"))
                                                                      (switch `/Game/Dialogue_System/E_DialogueState` _state_10
                                                                        (:`NewEnumerator0`
                                                                          (switch `int` _optionindex_8
                                                                            (:`0`
                                                                              (bind (_state_11 _optionindex_9) (`self.AddDialogue` "???" "And the formation of the two kingdoms." (`|MakeArray` "Are you talking about the Lineal Kingdom and the Colorful Kingdom?" :!type "Text") "/Engine/VREditor/Sounds/UI/Click_on_Button_Cue.Click_on_Button_Cue" "/Game/Asset_RPG/Blueprints/Basics/Personaje_2D/Sprites/Molly_NPC/AnimSequences/Idle.Idle"))
                                                                              (switch `/Game/Dialogue_System/E_DialogueState` _state_11
                                                                                (:`NewEnumerator0`
                                                                                  (switch `int` _optionindex_9
                                                                                    (:`0`
                                                                                      (bind (_state_12 _optionindex_10) (`self.AddDialogue` "Charlie" "(And what did he say about the universe?)" (`|MakeArray`) "/Engine/VREditor/Sounds/UI/Click_on_Button_Cue.Click_on_Button_Cue" "/Game/Asset_RPG/Blueprints/Basics/Personaje_2D/Sprites/Molly_NPC/AnimSequences/Idle.Idle"))
                                                                                      (switch `/Game/Dialogue_System/E_DialogueState` _state_12
                                                                                        (:`NewEnumerator0`
                                                                                          (switch `int` _optionindex_10
                                                                                            (:`0`
                                                                                              (bind (_state_13 _optionindex_11) (`self.AddDialogue` "???" "Yes. They weren’t always like that, they were one, one sole kingdom." (`|MakeArray` "(W-What is he saying…)" :!type "Text") "/Engine/VREditor/Sounds/UI/Click_on_Button_Cue.Click_on_Button_Cue" "/Game/Asset_RPG/Blueprints/Basics/Personaje_2D/Sprites/Molly_NPC/AnimSequences/Idle.Idle"))
                                                                                              (switch `/Game/Dialogue_System/E_DialogueState` _state_13
                                                                                                (:`NewEnumerator0`
                                                                                                  (switch `int` _optionindex_11
                                                                                                    (:`0`
                                                                                                      (bind (_state_14 _optionindex_12) (`self.AddDialogue` "???" "I could illustrate what happened." (`|MakeArray`) "/Engine/VREditor/Sounds/UI/Click_on_Button_Cue.Click_on_Button_Cue" "/Game/Asset_RPG/Blueprints/Basics/Personaje_2D/Sprites/Molly_NPC/AnimSequences/Idle.Idle"))
                                                                                                      (switch `/Game/Dialogue_System/E_DialogueState` _state_14
                                                                                                        (:`NewEnumerator0`
                                                                                                          (switch `int` _optionindex_12
                                                                                                            (:`0`
                                                                                                              (bind (_state_15 _optionindex_13) (`self.AddDialogue` "???" "If you're curious…" (`|MakeArray` "To tell the truth, it has caught my attention)" :!type "Text") "/Engine/VREditor/Sounds/UI/Click_on_Button_Cue.Click_on_Button_Cue" "/Game/Asset_RPG/Blueprints/Basics/Personaje_2D/Sprites/Molly_NPC/AnimSequences/Idle.Idle"))
                                                                                                              (switch `/Game/Dialogue_System/E_DialogueState` _state_15
                                                                                                                (:`NewEnumerator0`
                                                                                                                  (switch `int` _optionindex_13
                                                                                                                    (:`0`
                                                                                                                      (bind (_state_16 _optionindex_14) (`self.AddDialogue` "Charlie" "Well, there’s nothing more interesting around here…" (`|MakeArray`) "/Engine/VREditor/Sounds/UI/Click_on_Button_Cue.Click_on_Button_Cue" "/Game/Asset_RPG/Blueprints/Basics/Personaje_2D/Sprites/Molly_NPC/AnimSequences/Idle.Idle"))
                                                                                                                      (switch `/Game/Dialogue_System/E_DialogueState` _state_16
                                                                                                                        (:`NewEnumerator0`
                                                                                                                          (switch `int` _optionindex_14
                                                                                                                            (:`0`
                                                                                                                              (bind (_state_17 _optionindex_15) (`self.AddDialogue` "Charlie" "So tell me about it!" (`|MakeArray`) "/Engine/VREditor/Sounds/UI/Click_on_Button_Cue.Click_on_Button_Cue" "/Game/Asset_RPG/Blueprints/Basics/Personaje_2D/Sprites/Molly_NPC/AnimSequences/Idle.Idle"))
                                                                                                                              (switch `/Game/Dialogue_System/E_DialogueState` _state_17
                                                                                                                                (:`NewEnumerator0`
                                                                                                                                  (switch `int` _optionindex_15
                                                                                                                                    (:`0`
                                                                                                                                      (bind _state_18 (`self.AddDialogue` "???" "All right…" (`|MakeArray`) "/Engine/VREditor/Sounds/UI/Click_on_Button_Cue.Click_on_Button_Cue" "/Game/Asset_RPG/Blueprints/Basics/Personaje_2D/Sprites/Molly_NPC/AnimSequences/Idle.Idle"))
                                                                                                                                      (switch `/Game/Dialogue_System/E_DialogueState` _state_18
                                                                                                                                        (:`NewEnumerator0`
                                                                                                                                          (`self.SetDialogueBranch` "Normal")
                                                                                                                                          (`self.CloseConversation`))
                                                                                                                                        (:`NewEnumerator1`
                                                                                                                                          (`self.WBP_CutScene`
                                                                                                                                            (:`then`
                                                                                                                                              _)
                                                                                                                                            (:`else`
                                                                                                                                              (bind _returnvalue (`|CreateWidget` "/Game/Demo/Cinematica/Widget/WBP_Cinematica.WBP_Cinematica_C"))
                                                                                                                                              (set `self.WBP_CutScene` _returnvalue)))
                                                                                                                                          (`UserWidget.AddToViewport` (`self.WBP_CutScene`) 0)
                                                                                                                                          (`MediaPlayer.OpenSource` (`self.MediaPlayer`) (`self.MediaSource`))
                                                                                                                                          (`self.Delay`))))))))))))))))))))))))))))))))))))))))))))))))))))))))))))))))))))))