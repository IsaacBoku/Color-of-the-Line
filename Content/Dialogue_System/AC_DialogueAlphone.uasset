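; Dialogue component for the NPC Alphone, who gives Charlie a paid chore to clear rats from the sewers.
; It overrides the parent Dialogue function with a linear chain of AddDialogue lines, each advancing on Pass Through and, where offered, a single player reply.
; All lines sit under the default tree branch.
; The final line sets the dialogue branch to Normal with a progress value, then closes the conversation.
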(fn `Dialogue`
  (`parent.Dialogue`)
  (switch `name` (`self.ActiveTreeBranch`)
    (:`Default`
      (bind (_state _optionindex) (`self.AddDialogue` "Alphone" "Morning, Charlie." (`|MakeArray` "How’s it going Alphone. I’ll go straight to the point, Molly told me you wanted to give me a chore, isn’t that right?" :!type "Text") "/Engine/VREditor/Sounds/UI/Click_on_Button_Cue.Click_on_Button_Cue" "/Game/Asset_RPG/Blueprints/Basics/Personaje_2D/Sprites/Molly_NPC/AnimSequences/Idle.Idle"))
      (switch `/Game/Dialogue_System/E_DialogueState` _state
        (:`NewEnumerator0`
          (switch `int` _optionindex
            (:`0`
              (bind _state_2 (`self.AddDialogue` "Alphone" "Well… That’s about right." (`|MakeArray`) "/Engine/VREditor/Sounds/UI/Click_on_Button_Cue.Click_on_Button_Cue" "/Game/Asset_RPG/Blueprints/Basics/Personaje_2D/Sprites/Molly_NPC/AnimSequences/Idle.Idle"))
              (switch `/Game/Dialogue_System/E_DialogueState` _state_2
                (:`NewEnumerator0`
                  (bind _state_3 (`self.AddDialogue` "Alphone" "The rats are returning to the streets, and I can’t do the job. That’s why I wanted to ask you to do it. Don’t want them to be roaming around anymore." (`|MakeArray`) "/Engine/VREditor/Sounds/UI/Click_on_Button_Cue.Click_on_Button_Cue" "/Game/Asset_RPG/Blueprints/Basics/Personaje_2D/Sprites/Molly_NPC/AnimSequences/Idle.Idle"))
                  (switch `/Game/Dialogue_System/E_DialogueState` _state_3
                    (:`NewEnumerator0`
                      (bind (_state_4 _optionindex_2) (`self.AddDialogue` "Alphone" "I know it’s…… a little gross in the tunnels, but you’re the only young man I know who’s brave enough for this kind of situation." (`|MakeArray` "Color me shocked, I didn’t know you had such trust in me~" :!type "Text") "/Engine/VREditor/Sounds/UI/Click_on_Button_Cue.Click_on_Button_Cue" "/Game/Asset_RPG/Blueprints/Basics/Personaje_2D/Sprites/Molly_NPC/AnimSequences/Idle.Idle"))
                      (switch `/Game/Dialogue_System/E_DialogueState` _state_4
                        (:`NewEnumerator0`
                          (switch `int` _optionindex_2
                            (:`0`
                              (bind (_state_5 _optionindex_3) (`self.AddDialogue` "Alphone" "Argh! Don’t make me regret my decision…" (`|MakeArray` "Hehe, anyway, as long as you pay me well for this I’ll do the job in no time. Wouldn’t want to get dirty for nothing in return." :!type "Text") "/Engine/VREditor/Sounds/UI/Click_on_Button_Cue.Click_on_Button_Cue" "/Game/Asset_RPG/Blueprints/Basics/Personaje_2D/Sprites/Molly_NPC/AnimSequences/Idle.Idle"))
                              (switch `/Game/Dialogue_System/E_DialogueState` _state_5
                                (:`NewEnumerator0`
                                  (switch `int` _optionindex_3
                                    (:`0`
                                      (bind (_state_6 _optionindex_4) (`self.AddDialogue` "Alphone" "Yeah yeah, I’ll give you a good amount if you get rid of that pesky pest." (`|MakeArray` " Deal then. So, where can I find a way to get into the sewers?" :!type "Text") "/Engine/VREditor/Sounds/UI/Click_on_Button_Cue.Click_on_Button_Cue" "/Game/Asset_RPG/Blueprints/Basics/Personaje_2D/Sprites/Molly_NPC/AnimSequences/Idle.Idle"))
                                      (switch `/Game/Dialogue_System/E_DialogueState` _state_6
                                        (:`NewEnumerator0`
                                          (switch `int` _optionindex_4
                                            (:`0`
                                              (bind (_state_7 _optionindex_5) (`self.AddDialogue` "Alphone" "You’ll need to follow that path over there until you find a backstreet. There you’ll see an opened manhole cover, from there you just go down the ladder and try to find the rats as soon as possible." (`|MakeArray` "Great, I’ll see you later for the compensation then!" :!type "Text") "/Engine/VREditor/Sounds/UI/Click_on_Button_Cue.Click_on_Button_Cue" "/Game/Asset_RPG/Blueprints/Basics/Personaje_2D/Sprites/Molly_NPC/AnimSequences/Idle.Idle"))
                                              (switch `/Game/Dialogue_System/E_DialogueState` _state_7
                                                (:`NewEnumerator0`
                                                  (switch `int` _optionindex_5
                                                    (:`0`
                                                      (bind _state_8 (`self.AddDialogue` "Alphone" "Ugh, fine, just go already!" (`|MakeArray`) "/Engine/VREditor/Sounds/UI/Click_on_Button_Cue.Click_on_Button_Cue" "/Game/Asset_RPG/Blueprints/Basics/Personaje_2D/Sprites/Molly_NPC/AnimSequences/Idle.Idle"))
                                                      (switch `/Game/Dialogue_System/E_DialogueState` _state_8
                                                        (:`NewEnumerator0`
                                                          (`self.SetDialogueBranch` "Normal")
                                                          (`self.CloseConversation`))))))))))))))))))))))))))))))