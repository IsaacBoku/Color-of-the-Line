(fn `Dialogue`
  (`parent.Dialogue`)
  (switch `name` (`self.ActiveTreeBranch`)
    (:`Morning`
      (bind _state (`self.AddDialogue` "Alphone" "Good morning" (`|MakeArray`)))
      (switch `/Game/Dialogue_System/E_DialogueState` _state
        (:`NewEnumerator0`
          (`self.ClearDialogueProgress`)
          (`self.CloseConversation`))))
    (:`Afternoon`
      (if (`self.HasGivenBread?`)
        (bind _state_2 (`self.AddDialogue` "Alphone" "thank you " (`|MakeArray`)))
        (switch `/Game/Dialogue_System/E_DialogueState` _state_2
          (:`NewEnumerator0`
            (`self.ClearDialogueProgress`)
            (`self.CloseConversation`)))
        (else
          (bind (_state_3 _optionindex) (`self.AddDialogue` "Alphone" "i would love a piece of bread, i've not eaten all day. CAn you get me one?" (`|MakeArray` "Sure" "No" :!type "Text")))
          (switch `/Game/Dialogue_System/E_DialogueState` _state_3
            (:`NewEnumerator0`
              (switch `int` _optionindex
                (:`0`
                  (bind _state_4 (`self.AddDialogue` "Alphone" "Great" (`|MakeArray`)))
                  (switch `/Game/Dialogue_System/E_DialogueState` _state_4
                    (:`NewEnumerator0`
                      (if true
                        (bind (_state_5 _optionindex_2) (`self.AddDialogue` "Alphone" "ahh i see you have bread, can i have it please" (`|MakeArray` "Sure" "no" :!type "Text")))
                        (switch `/Game/Dialogue_System/E_DialogueState` _state_5
                          (:`NewEnumerator0`
                            (switch `int` _optionindex_2
                              (:`0`
                                (bind _state_6 (`self.AddDialogue` "Alphone" "ahh wonderful" (`|MakeArray`)))
                                (switch `/Game/Dialogue_System/E_DialogueState` _state_6
                                  (:`NewEnumerator0`
                                    (`self.ClearDialogueProgress`)
                                    (`self.CloseConversation`))
                                  (:`NewEnumerator1`
                                    (set `self.HasGivenBread?` true))))
                              (:`1`
                                (bind _state_7 (`self.AddDialogue` "Alphone" "oh, ok" (`|MakeArray`)))
                                (switch `/Game/Dialogue_System/E_DialogueState` _state_7
                                  (:`NewEnumerator0`
                                    (`self.RemoveDIalogueProcess` 2)
                                    (`self.CloseConversation`)))))))
                        (else
                          (bind _state_8 (`self.AddDialogue` "Alphone" "Come speak to me, when you have the bread" (`|MakeArray`)))
                          (switch `/Game/Dialogue_System/E_DialogueState` _state_8
                            (:`NewEnumerator0`
                              (`self.RemoveDIalogueProcess` 1)
                              (`self.CloseConversation`))))))))
                (:`1`
                  (bind _state_9 (`self.AddDialogue` "Alphone" "ahh okey" (`|MakeArray`)))
                  (switch `/Game/Dialogue_System/E_DialogueState` _state_9
                    (:`NewEnumerator0`
                      (`self.ClearDialogueProgress`)
                      (`self.CloseConversation`))))))))))
    (:`Night`
      (bind _state_10 (`self.AddDialogue` "Alphone" "ahh, i'm trying to sleep, leave me alone." (`|MakeArray`)))
      (switch `/Game/Dialogue_System/E_DialogueState` _state_10
        (:`NewEnumerator0`
          (`self.ClearDialogueProgress`)
          (`self.CloseConversation`))))))

(fn `OpenConversation`
  (`self.SetDialogueBranch` "None")
  (`parent.OpenConversation`))