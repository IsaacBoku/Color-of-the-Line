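; BP_QuestGiver is a quest-giving actor that plays a dialogue, then offers its list of quests.
; A trigger radius shows or hides an interaction widget for the 2D world character, and Tick rotates that widget toward the player camera.
; Each Interact call advances the dialogue; running past the last line opens a quest widget filled from the Quests array.
; Interacting again or calling Closewidget removes it and restores game-only input.
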(event `self.TriggerRadius.OnComponentBeginOverlap`
  (params (OverlappedComponent :type "PrimitiveComponent Object Reference") (OtherActor :type "Actor Object Reference") (OtherComp :type "PrimitiveComponent Object Reference") (OtherBodyIndex :type Integer) (bFromSweep :type Boolean) (SweepResult :type "HitResult Structure (by ref)"))
  (cast `/Game/Asset_RPG/Blueprints/Basics/Personaje_2D/BP_Character_World_2D` OtherActor)
  (`SceneComponent.SetVisibility` (`self.InteractionWidget`) true false))

(event `self.ReceiveTick`
  (params (DeltaSeconds :type "Float (single-precision)"))
  (`SceneComponent.K2_SetWorldRotation` (`self.InteractionWidget`) (`KismetMathLibrary.FindLookAtRotation` (`SceneComponent.K2_GetComponentLocation` (`self.InteractionWidget`)) (`SceneComponent.K2_GetComponentLocation` (`PlayerCameraManager.TransformComponent` (`GameplayStatics.GetPlayerCameraManager` 0)))) false false))

(event `self.TriggerRadius.OnComponentEndOverlap`
  (params (OverlappedComponent :type "PrimitiveComponent Object Reference") (OtherActor :type "Actor Object Reference") (OtherComp :type "PrimitiveComponent Object Reference") (OtherBodyIndex :type Integer))
  (cast `/Game/Asset_RPG/Blueprints/Basics/Personaje_2D/BP_Character_World_2D` OtherActor)
  (`SceneComponent.SetVisibility` (`self.InteractionWidget`) false false))

(event `Open Quests Widget`
  (bind _returnvalue (`|GenericCreateObject` "/Game/Quest_System/WBP_QuestGiver.WBP_QuestGiver_C"))
  (bind _output_get (set `self.QuestWidget` _returnvalue))
  (`UserWidget.AddToViewport` _output_get 0)
  (set `self.WidgetActive` true)
  (set `/Game/Quest_System/WBP_QuestGiver.QuestGiverBP` self (`self.QuestWidget`))
  (for _array_element (`self.Quests`)
    (`/Game/Quest_System/WBP_QuestGiver.Add Quest` (`self.QuestWidget`) _array_element)))

(event `/Game/Quest_System/BPI_QuestGiver.Interact`
  (bind _returnvalue (`GameplayStatics.GetPlayerController` 0))
  (bind _returnvalue_2 (`GameplayStatics.GetPlayerController` 0))
  (if (not (`self.WidgetActive`))
    (if (not (`self.DialogueOpened?`))
      (bind _returnvalue_3 (`|CreateWidget` "/Game/Quest_System/WBP_QuestGIverDialogue.WBP_QuestGIverDialogue_C"))
      (bind _output_get (set `self.Dialogue_Widget` _returnvalue_3))
      (`UserWidget.AddToViewport` _output_get 0)
      (set `self.DialogueOpened?` true)
      (`TextBlock.SetText` (`/Game/Quest_System/WBP_QuestGIverDialogue.DialogueText` (`self.Dialogue_Widget`)) (`KismetTextLibrary.Conv_StringToText` (`|GetArrayItem` (`self.Dialogue`) (`self.DialogueIndex`))))
      (`/Engine/EditorBlueprintResources/StandardMacros.IncrementInt` (`self.DialogueIndex`)
        (:`  `
          (set `PlayerController.bShowMouseCursor` true _returnvalue_2)
          (`WidgetBlueprintLibrary.SetInputMode_GameAndUIEx` _returnvalue_2 (`self.QuestWidget`))))
      (else
        (`TextBlock.SetText` (`/Game/Quest_System/WBP_QuestGIverDialogue.DialogueText` (`self.Dialogue_Widget`)) (`KismetTextLibrary.Conv_StringToText` (`|GetArrayItem` (`self.Dialogue`) (`self.DialogueIndex`))))
        (`/Engine/EditorBlueprintResources/StandardMacros.IncrementInt` (`self.DialogueIndex`)
          (:`  `
            (if (> (`self.DialogueIndex`) (`KismetArrayLibrary.Array_Length` (`self.Dialogue`)))
              (`Widget.RemoveFromParent` (`self.Dialogue_Widget`))
              (set `self.Dialogue_Widget` null)
              (set `self.DialogueIndex` 0)
              (set `self.DialogueOpened?` false)
              (`self.Open Quests Widget`))))))
    (else
      (`Widget.RemoveFromParent` (`self.QuestWidget`) :!label _label)
      (set `self.QuestWidget` null)
      (set `PlayerController.bShowMouseCursor` false _returnvalue)
      (`WidgetBlueprintLibrary.SetInputMode_GameOnly` _returnvalue)
      (set `self.WidgetActive` false))))

(event `Close widget`
  (goto _label))

(fn `UserConstructionScript`)