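; Quest component that tracks the active quest's objectives and mirrors progress on a WBP_QuestHud widget it creates at BeginPlay.
; Events push the quest name and objective list to the HUD.
; EliminateEnemy empties a working copy of an objective's target actors, while Openchest matches the opened chest, each marking objectives completed by reference.
; Each completion increments a counter that, upon reaching the objective count, clears the quest and plays the HUD completion animation.
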(event `self.ReceiveBeginPlay`
  (bind _returnvalue (`|CreateWidget` "/Game/Quest_System/WBP_QuestHud.WBP_QuestHud_C"))
  (bind _output_get (set `self.QuestHUD Widget` _returnvalue))
  (`UserWidget.AddToViewport` _output_get 0)
  (`/Game/Quest_System/WBP_QuestHud.Hide Quest Panel` (`self.QuestHUD Widget`)))

(event `Set Active Quest Text`
  (`TextBlock.SetText` (`/Game/Quest_System/WBP_QuestHud.Active_Quest_text` (`self.QuestHUD Widget`)) (`KismetTextLibrary.Conv_StringToText` (`.Name_2_101801CE4F4EDF3098B7CA80D74F77DB` (break `/Game/Quest_System/S_Quest` (`self.ActiveQuest`)))))
  (`/Game/Quest_System/WBP_QuestHud.Show Quest Panel` (`self.QuestHUD Widget`)))

(event `Set Objectives`
  (bind (_activequest_name _activequest_description _activequest_secundary _activequest_completed _activequest_objectives) (break `/Game/Quest_System/S_Quest` (`self.ActiveQuest`)))
  (`/Game/Quest_System/WBP_QuestHud.Fill Objectives` (`self.QuestHUD Widget`) _activequest_objectives))

(event `Eliminate Enemy`
  (params (`Enemy eliminated` :type "Actor Object Reference"))
  (bind (_activequest_name _activequest_description _activequest_secundary _activequest_completed _activequest_objectives) (break `/Game/Quest_System/S_Quest` (`self.ActiveQuest`)))
  (bind _returnvalue (`KismetArrayLibrary.Array_Length` (`self.Enemy actors array`)))
  (for _array_element _activequest_objectives
    (bind (_nameaim _completed _actorstoeliminate _chesttoopen _iseliminateenemyobjetive _ischestobjetive) (break `/Game/Quest_System/S_QuestObjetive` _array_element))
    (if (and (not _completed) _iseliminateenemyobjetive)
      (if (not (!= (`KismetArrayLibrary.Array_Length` (`self.Enemy actors array`)) 0))
        (bind _output_get (set `self.Enemy actors array` _actorstoeliminate)))
      (`KismetArrayLibrary.Array_RemoveItem` _output_get `Enemy eliminated`)
      (`|VariableSetRef` _array_element (make `/Game/Quest_System/S_QuestObjetive` _nameaim false (`self.Enemy actors array`) _chesttoopen _iseliminateenemyobjetive _ischestobjetive))
      (`KismetSystemLibrary.PrintString` (`KismetStringLibrary.Conv_IntToString` _returnvalue))
      (if (== _returnvalue 0)
        (`|VariableSetRef` _array_element (make `/Game/Quest_System/S_QuestObjetive` _nameaim true _ _chesttoopen _iseliminateenemyobjetive _ischestobjetive))
        (`/Game/Quest_System/WBP_QuestHud.Complete Objectives` (`self.QuestHUD Widget`) _array_element)
        (`self.Objetive Completed`)
        (`KismetSystemLibrary.PrintString` "Completed")))))

(event `Open chest`
  (params (Chest :type "Actor Object Reference"))
  (bind (_activequest_name _activequest_description _activequest_secundary _activequest_completed _activequest_objectives) (break `/Game/Quest_System/S_Quest` (`self.ActiveQuest`)))
  (for _array_element _activequest_objectives
    (bind (_nameaim _completed _actorstoeliminate _chesttoopen _iseliminateenemyobjetive _ischestobjetive) (break `/Game/Quest_System/S_QuestObjetive` _array_element))
    (if (and _ischestobjetive (== Chest _chesttoopen))
      (`|VariableSetRef` _array_element (make `/Game/Quest_System/S_QuestObjetive` _nameaim true _actorstoeliminate null _iseliminateenemyobjetive _ischestobjetive))
      (`/Game/Quest_System/WBP_QuestHud.Complete Objectives` (`self.QuestHUD Widget`) _array_element)
      (`self.Objetive Completed`)
      (`KismetSystemLibrary.PrintString` "Completed"))))

(event `Objetive Completed`
  (bind (_activequest_name _activequest_description _activequest_secundary _activequest_completed _activequest_objectives) (break `/Game/Quest_System/S_Quest` (`self.ActiveQuest`)))
  (`/Engine/EditorBlueprintResources/StandardMacros.IncrementInt` (`self.Objetives Completed`)
    (:`  `
      (if (>= (`self.Objetives Completed`) (`KismetArrayLibrary.Array_Length` _activequest_objectives))
        (`KismetSystemLibrary.PrintString` "Quest completed")
        (set `self.ActiveQuest` (struct))
        (set `self.Objetives Completed` 0)
        (`/Game/Quest_System/WBP_QuestHud.Play Quest Completed Animation` (`self.QuestHUD Widget`))))))